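; Player controller for a cursor-aimed shooter, handling pawn movement, shooting and reloading.
; Tick sums the WASD axis values into world-space movement input on the X/Y plane, scaled by MovementSpeed and delta time.
; Shoot traces under the cursor, flattens the target to pawn height, and passes the weapon an offset position and rotation along that aim.
; Shoot and Reload both reach the Weapon by casting the player pawn.
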(event `self.ReceiveTick`
  (params (DeltaSeconds :type "Float (single-precision)"))
  ;[0 0.2265 1] WASD Movement
  (`Pawn.AddMovementInput` (`self.K2_GetPawn`) (`KismetMathLibrary.MakeVector` (+ (`self.GetInputAxisValue`) (`self.GetInputAxisValue`)) (+ (`self.GetInputAxisValue`) (`self.GetInputAxisValue`))) (* DeltaSeconds (`self.Movement Speed`)) false))

(event `InputAction|Shoot`
  (bind _returnvalue (`self.K2_GetActorLocation` (`self.K2_GetPawn`)))
  (bind _returnvalue_2 (`KismetMathLibrary.GetDirectionVector` _returnvalue (`KismetMathLibrary.MakeVector` (.x (`GameplayStatics.BreakHitResult` (`self.GetHitResultUnderCursorByChannel` "TraceTypeQuery1"))) (.y (`GameplayStatics.BreakHitResult` (`self.GetHitResultUnderCursorByChannel` "TraceTypeQuery1"))) (.z _returnvalue))))
  ;[1 0.01618 0] Shoot
  (:`Pressed`
    (bind _aspawn_c (cast `/Game/Blueprints/Game/Pawn` (`GameplayStatics.GetPlayerPawn` 0)))
    (`/Game/Blueprints/Game/Weapon.Shoot` (`/Game/Blueprints/Game/Pawn.Weapon` _aspawn_c) (+ _returnvalue (* _returnvalue_2 75.0)) (`KismetMathLibrary.Conv_VectorToRotator` _returnvalue_2))))

(event `InputAction|Reload`
  ;[1 1 1] Reload
  (:`Pressed`
    (bind _aspawn_c (cast `/Game/Blueprints/Game/Pawn` (`GameplayStatics.GetPlayerPawn` 0)))
    (`/Game/Blueprints/Game/Weapon.Reload` (`/Game/Blueprints/Game/Pawn.Weapon` _aspawn_c))))

(fn `UserConstructionScript`)