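; Enemy pawn that chases the nearest Pawn, intended to be a player, and is destroyed when its life runs out.
; Every Tick it scans all Pawns by distance, with no filter for players or itself, and stores the closest one's location.
; It then sends its controller there with SimpleMoveToLocation.
; AnyDamage subtracts damage from Life and destroys the actor at zero or below.
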(event `self.ReceiveTick`
  (params (DeltaSeconds :type "Float (single-precision)"))
  (set `self.ShortestDistance` 100000.0)
  ;[1 1 1] For each player
  (bind _outactors (`GameplayStatics.GetAllActorsOfClass` "/Game/Blueprints/Game/Pawn.Pawn_C"))
  (for _array_element _outactors
    ;[1 1 1] Get closest player and his position
    (bind _returnvalue (`self.GetDistanceTo` _array_element self))
    (if (< _returnvalue (`self.ShortestDistance`))
      (set `self.ShortestDistance` _returnvalue)
      (set `self.Destination` (`self.K2_GetActorLocation` _array_element))))
  ;[1 1 1] Run to player
  (`NavigationSystem.SimpleMoveToLocation` (`Pawn.GetController` self) (`self.Destination`)))

(event `self.ReceiveAnyDamage`
  (params (Damage :type "Float (single-precision)") (DamageType :type "DamageType Object Reference") (InstigatedBy :type "Controller Object Reference") (DamageCauser :type "Actor Object Reference"))
  (bind _life (`self.Life`))
  ;[1 1 1] Take damage
  (set `self.Life` (- _life Damage))
  (if (<= _life 0.0)
    (`self.K2_DestroyActor`)))

(fn `UserConstructionScript`)