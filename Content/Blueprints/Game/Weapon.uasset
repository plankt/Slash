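; Weapon is a Blueprint that fires P_Ball projectiles from a limited clip and handles reloading.
; Shoot spawns a ball at the given position and rotation, spending one round, if ammo remains, no reload is running and the fire cooldown has passed.
; Fire rate and reload use game-time timestamps instead of timers, with Tick refilling the clip once the reload time elapses.
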(event `Shoot`
  (params (Position :type "Object.Vector Structure") (Rotation :type "Object.Rotator Structure"))
  ;[1 1 1] Shooting
  (if (> (`self.AmmoInClip`) 0.0)
    (if (`self.Reloading`)
      _
      (elif (>= (`KismetSystemLibrary.GetGameTimeInSeconds`) (`self.FireCD`))
        (set `self.FireCD` (+ (`KismetSystemLibrary.GetGameTimeInSeconds`) (`self.RateOfFire`)))
        (set `self.AmmoInClip` (- (`self.AmmoInClip`) 1.0))
        (`|SpawnActorFromClass` "/Game/Props/Projectiles/P_Ball.P_Ball_C" (`KismetMathLibrary.MakeTransform` Position Rotation))))))

(event `Reload`
  ;[1 1 1] Reloading
  (if (not (`self.Reloading`))
    (set `self.ReloadCD` (+ (`KismetSystemLibrary.GetGameTimeInSeconds`) (`self.ReloadTime`)))
    (set `self.Reloading` true)))

(event `self.ReceiveTick`
  (params (DeltaSeconds :type "Float (single-precision)"))
  ;[1 1 1] Reloading
  (if (`self.Reloading`)
    (if (>= (`KismetSystemLibrary.GetGameTimeInSeconds`) (`self.ReloadCD`))
      (set `self.Reloading` false)
      (set `self.AmmoInClip` (`self.ClipSize`)))))

(fn `UserConstructionScript`)